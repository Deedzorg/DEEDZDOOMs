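; Barn actor with four doors that the player slides open or closed by pressing E while inside each door's trigger volume.
; Each volume's overlap enables input and opens that door's Gate, and leaving disables input and closes it.
; A gated E press plays the door's timeline, or reverses it if fully open, lerping relative location between start and end vectors.
; The logic is duplicated per door.
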(event OnComponentBeginOverlap(dooroverlay)
  (params (OverlappedComponent :type Primitive%20Component%20Object%20Reference) (OtherActor :type Actor%20Object%20Reference) (OtherComp :type Primitive%20Component%20Object%20Reference) (OtherBodyIndex :type Integer) (bFromSweep :type Boolean) (SweepResult :type Hit%20Result%20Structure%20%28by%20ref%29))
  (Input|EnableInput (Game|GetPlayerController 0))
  ;[1 1 1] open door1
  (Utilities|FlowControl|Gate true) ; enters at Open
)

(event OnComponentEndOverlap(dooroverlay)
  (params (OverlappedComponent :type Primitive%20Component%20Object%20Reference) (OtherActor :type Actor%20Object%20Reference) (OtherComp :type Primitive%20Component%20Object%20Reference) (OtherBodyIndex :type Integer))
  (Input|DisableInput (Game|GetPlayerController 0))
  ;[1 1 1] open door1
  (Utilities|FlowControl|Gate true) ; enters at Close
)

(event OnComponentBeginOverlap(door2overlay)
  (params (OverlappedComponent :type Primitive%20Component%20Object%20Reference) (OtherActor :type Actor%20Object%20Reference) (OtherComp :type Primitive%20Component%20Object%20Reference) (OtherBodyIndex :type Integer) (bFromSweep :type Boolean) (SweepResult :type Hit%20Result%20Structure%20%28by%20ref%29))
  (Input|EnableInput (Game|GetPlayerController 0))
  ;[1 1 1] door2 open
  (Utilities|FlowControl|Gate true) ; enters at Open
)

(event OnComponentEndOverlap(door2overlay)
  (params (OverlappedComponent :type Primitive%20Component%20Object%20Reference) (OtherActor :type Actor%20Object%20Reference) (OtherComp :type Primitive%20Component%20Object%20Reference) (OtherBodyIndex :type Integer))
  (Input|DisableInput (Game|GetPlayerController 0))
  ;[1 1 1] door2 open
  (Utilities|FlowControl|Gate true) ; enters at Close
)

(event OnComponentBeginOverlap(door3overlay)
  (params (OverlappedComponent :type Primitive%20Component%20Object%20Reference) (OtherActor :type Actor%20Object%20Reference) (OtherComp :type Primitive%20Component%20Object%20Reference) (OtherBodyIndex :type Integer) (bFromSweep :type Boolean) (SweepResult :type Hit%20Result%20Structure%20%28by%20ref%29))
  (Input|EnableInput (Game|GetPlayerController 0))
  ;[1 1 1] door 3 open
  (Utilities|FlowControl|Gate true) ; enters at Open
)

(event OnComponentEndOverlap(door3overlay)
  (params (OverlappedComponent :type Primitive%20Component%20Object%20Reference) (OtherActor :type Actor%20Object%20Reference) (OtherComp :type Primitive%20Component%20Object%20Reference) (OtherBodyIndex :type Integer))
  (Input|DisableInput (Game|GetPlayerController 0))
  ;[1 1 1] door 3 open
  (Utilities|FlowControl|Gate true) ; enters at Close
)

(event OnComponentBeginOverlap(door4overlay)
  (params (OverlappedComponent :type Primitive%20Component%20Object%20Reference) (OtherActor :type Actor%20Object%20Reference) (OtherComp :type Primitive%20Component%20Object%20Reference) (OtherBodyIndex :type Integer) (bFromSweep :type Boolean) (SweepResult :type Hit%20Result%20Structure%20%28by%20ref%29))
  (Input|EnableInput (Game|GetPlayerController 0))
  ;[1 1 1] door4 open
  (Utilities|FlowControl|Gate true) ; enters at Open
)

(event OnComponentEndOverlap(door4overlay)
  (params (OverlappedComponent :type Primitive%20Component%20Object%20Reference) (OtherActor :type Actor%20Object%20Reference) (OtherComp :type Primitive%20Component%20Object%20Reference) (OtherBodyIndex :type Integer))
  (Input|DisableInput (Game|GetPlayerController 0))
  ;[1 1 1] door4 open
  (Utilities|FlowControl|Gate true) ; enters at Close
)

(event Collision|EventActorBeginOverlap
  (params (OtherActor :type Actor%20Object%20Reference)))

(event EventTick
  (params (DeltaSeconds :type Float%20%28single-precision%29)))

(event EventBeginPlay
  ;[1 1 1] sets the inistail door location
)

(event Input|KeyboardEvents|E
  (params (Key :type Key%20Structure)))

(event Input|KeyboardEvents|E
  (params (Key :type Key%20Structure))
  ;[1 1 1] door4 open
  (:Pressed
    (Utilities|FlowControl|Gate true
      (:Exit
        (if (< (stale _opendoor) 1.0)
          (bind _opendoor (Timeline|Timeline_2 Play)
            (:Update
              (Transformation|SetRelativeLocation (Variables|Default|Getdoor4) (Math|Vector|Lerp(Vector) (Variables|Default|Getdoor4startpos_0) (Variables|Default|Getdoor4endpos_1) _opendoor) false false)))
          (else
            (Timeline|Timeline_2 Reverse)))))))

(event Input|KeyboardEvents|E
  (params (Key :type Key%20Structure))
  ;[1 1 1] open door1
  (:Pressed
    (Utilities|FlowControl|Gate true
      (:Exit
        (if (< (stale _opendoor) 1.0)
          (bind _opendoor (Timeline|opendoor Play)
            (:Update
              (Transformation|SetRelativeLocation (Variables|Default|Getbarndoor) (Math|Vector|Lerp(Vector) (Variables|Default|Getdoor1startpos) (Variables|Default|Getdoor1endpos) _opendoor) false false)))
          (else
            (Timeline|opendoor Reverse)))))))

(event Input|KeyboardEvents|E
  (params (Key :type Key%20Structure))
  ;[1 1 1] door2 open
  (:Pressed
    (Utilities|FlowControl|Gate true
      (:Exit
        (if (< (stale _opendoor) 1.0)
          (bind _opendoor (Timeline|Timeline_0 Play)
            (:Update
              (Transformation|SetRelativeLocation (Variables|Default|Getdoor2) (Math|Vector|Lerp(Vector) (Variables|Default|Getdoor2startpos_0) (Variables|Default|Getdoor2endpos_0) _opendoor) false false)))
          (else
            (Timeline|Timeline_0 Reverse)))))))

(event Input|KeyboardEvents|E
  (params (Key :type Key%20Structure))
  (:Pressed
    ;[1 1 1] door 3 open
    (Utilities|FlowControl|Gate true
      (:Exit
        (if (< (stale _opendoor) 1.0)
          (bind _opendoor (Timeline|Timeline_1 Play)
            (:Update
              (Transformation|SetRelativeLocation (Variables|Default|Getdoor3) (Math|Vector|Lerp(Vector) (Variables|Default|Getdoor3startpos_1) (Variables|Default|Getdoor3endpos_0) _opendoor) false false)))
          (else
            (Timeline|Timeline_1 Reverse)))))))

(fn ConstructionScript)