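; Interactable secret block that slides its Jumpbox between two relative positions when the player presses Interact nearby.
; Overlapping Box enables input and opens a gate; leaving disables both.
; Interact plays or reverses a timeline that lerps the Jumpbox location, depending on its current value.
; A second gate fires a meme sound and "u found me" message on timeline update, closes itself, then reopens when the timeline finishes.
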(event OnComponentBeginOverlap(Box)
  (params (OverlappedComponent :type Primitive%20Component%20Object%20Reference) (OtherActor :type Actor%20Object%20Reference) (OtherComp :type Primitive%20Component%20Object%20Reference) (OtherBodyIndex :type Integer) (bFromSweep :type Boolean) (SweepResult :type Hit%20Result%20Structure%20%28by%20ref%29))
  (Input|EnableInput (Game|GetPlayerController 0))
  ;[1 1 1] door4 open
  (Utilities|FlowControl|Gate true) ; enters at Open
)

(event OnComponentEndOverlap(Box)
  (params (OverlappedComponent :type Primitive%20Component%20Object%20Reference) (OtherActor :type Actor%20Object%20Reference) (OtherComp :type Primitive%20Component%20Object%20Reference) (OtherBodyIndex :type Integer))
  (Input|DisableInput (Game|GetPlayerController 0))
  ;[1 1 1] door4 open
  (Utilities|FlowControl|Gate true) ; enters at Close
)

(event EventBeginPlay)

(event Collision|EventActorBeginOverlap
  (params (OtherActor :type Actor%20Object%20Reference)))

(event EventTick
  (params (DeltaSeconds :type Float%20%28single-precision%29)))

(event Input|ActionEvents|InputActionInteract
  (params (Key :type Key%20Structure))
  (:Pressed
    ;[1 1 1] door4 open
    (Utilities|FlowControl|Gate true
      (:Exit
        (if (< (stale _opendoor) 1.0)
          (bind _opendoor (Timeline|Timeline_0 Play)
            (:Update
              (Transformation|SetRelativeLocation (Variables|Default|Getjumpbox) (Math|Vector|Lerp(Vector) (Variables|Default|GetNewVar_0) (Variables|Default|GetNewVar_1) _opendoor) false false)
              (Utilities|FlowControl|Gate true :!label _label
                (:Exit
                  (Audio|PlaySound2D "/Game/Blueprints/DAMN_SON_WHERED_YOU_FIND_THIS.DAMN_SON_WHERED_YOU_FIND_THIS" 1.0 1.0 0.0 0 0)
                  (Development|PrintString "u found me")
                  (goto _label Close))))
            (:Finished
              (goto _label Open)))
          (else
            (Timeline|Timeline_0 Reverse)))))))

(fn ConstructionScript)